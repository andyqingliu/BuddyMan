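; GA_Jump is a Gameplay Ability that plays a jump animation montage for BuddyMan characters.
; On activation it commits, casts the avatar to BM_CharacterBase and picks the Ghoul or Zombie montage from its CharacterType, with debug prints along the way.
; It plays the montage through a wait task and ends on completion, blend out, interruption or cancellation.
; The graph applies no jump movement itself.
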(event Ability|EventActivateAbility
  (Ability|CommitAbility)
  (Development|PrintString "Active Jump GA ....")
  (bind _asbm_character_base (Utilities|Casting|CastToBM_CharacterBase (Ability|GetAvatarActorfromActorInfo)))
  (Development|PrintString (Utilities|String|Append "CharacterType=" (Utilities|String|EnumtoString (Variables|/Script/BuddyMan.BM_CharacterBase|GetCharacterType _asbm_character_base)) "Will use this AM."))
  (switch Utilities|FlowControl|Switch|SwitchonECharacterType (Variables|/Script/BuddyMan.BM_CharacterBase|GetCharacterType _asbm_character_base)
    (:Ghoul
      (Variables|Default|SetCur_AM_Jump (Variables|Default|GetAM_Ghoul_Jump)))
    (:Zombie
      (Variables|Default|SetCur_AM_Jump (Variables|Default|GetAM_Zombie_Jump))))
  (|PlayMontageandWaitProxy "None" (Variables|Default|GetCur_AM_Jump) 1.0 "None" true 1.0 0.0
    (:OnCompleted
      _)
    (:OnBlendOut
      _)
    (:OnInterrupted
      _)
    (:OnCancelled
      _))
  (Ability|EndAbility))

(event Ability|EventOnEndAbility
  (params (bWasCancelled :type Boolean)))