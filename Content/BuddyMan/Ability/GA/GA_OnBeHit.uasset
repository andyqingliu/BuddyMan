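; GA_OnBeHit is an event-triggered gameplay ability that plays a hit reaction on the owning BM_CharacterBase.
; It commits, then turns the owner to face the event's instigator on the horizontal plane.
; The character type from the current player state's info selects the Ghoul or Zombie hit montage.
; PlayMontageAndWaitForEvent plays it, and the ability ends on blend out, interruption or cancellation.
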(event Ability|EventOnEndAbility
  (params (bWasCancelled :type Boolean))
  (|CallParentFunction bWasCancelled) ; This node is disabled and will not be called.\nDrag off pins to build functionality.
)

(event Ability|EventActivateAbilityFromEvent
  (params (EventData :type Gameplay%20Event%20Data%20Structure%20%28by%20ref%29))
  (bind _instigator (Utilities|Struct|BreakGameplayEventData EventData))
  (bind _returnvalue (Ability|GetOwningActorfromActorInfo))
  (bind _returnvalue_2 (Transformation|GetActorLocation _instigator))
  (bind _returnvalue_3 (Transformation|GetActorLocation _returnvalue))
  (bind (_x _y) (Math|Vector|BreakVector _returnvalue_2))
  (Development|PrintString "GA_OnBeHit is call ....")
  (Ability|CommitAbility)
  (bind _asbm_character_base (Utilities|Casting|CastToBM_CharacterBase _returnvalue))
  (Transformation|SetActorRotation _returnvalue (Math|Rotator|FindLookatRotation _returnvalue_3 (Math|Vector|MakeVector _x _y (.Z (Math|Vector|BreakVector _returnvalue_3)))))
  (switch Utilities|FlowControl|Switch|SwitchonECharacterType (Utilities|Enum|ByteToEnumECharacterType (Math|Conversions|ToByte(Integer) (.playertype (Variables|/Script/BuddyMan.BM_PlayerStateBase|GetPlayerInfo (Variables|/Script/BuddyMan.BM_CharacterBase|GetCurPlayerState _asbm_character_base)))))
    (:Ghoul
      (Variables|Default|SetCurBeHitAM (Variables|Default|GetAM_Ghoul_BeHit)))
    (:Zombie
      (Variables|Default|SetCurBeHitAM (Variables|Default|GetAM_Zombie_BeHit))))
  (|PlayMontageandWaitforEvent "None" (Variables|Default|GetCurBeHitAM) "(GameplayTags=((TagName=\"Event.Montage\")))" 1.0 "None" true 1.0
    (:OnBlendOut
      _)
    (:OnInterrupted
      _)
    (:OnCancelled
      _))
  (Ability|EndAbility))