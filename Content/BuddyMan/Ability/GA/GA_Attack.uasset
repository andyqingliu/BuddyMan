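; Melee attack Gameplay Ability for BM_CharacterBase characters, with separate left and right montages for Ghoul and Zombie types.
; On activation, a forward box trace finds enemies, and the owner turns to face the first one.
; A right-vector dot product, taken after that turn, picks the montage side, defaulting to left without targets.
; The montage's Event.Montage event applies GE_BeHit to that enemy and sends it Ability.BeHit.
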(event EventActivateAbility
  (Development|PrintString "Receive ga_attack event")
  (bind _outactor (CallFunction|FindNearbyEnemy))
  (if (> (Utilities|Array|Length _outactor) 0)
    (CallFunction|RotatetoEnemy (Utilities|Array|Get(acopy) _outactor))
    (bind _bisleft (CallFunction|CalcEnemyDirection (Utilities|Array|Get(acopy) _outactor)))
    (CallFunction|InitCurMontagetbyEnemySide _bisleft)
    (else
      (Development|PrintString "Not has enemy....")
      (CallFunction|InitCurMontagetbyEnemySide true)))
  (|PlayMontageandWaitforEvent "None" (Variables|Default|GetCurMontage) "(GameplayTags=((TagName=\"Event.Montage\")))" 1.0 "None" true 1.0
    (:OnBlendOut
      (Ability|EndAbility :!label _label))
    (:OnInterrupted
      (goto _label))
    (:OnCancelled
      (goto _label))
    (:EventReceived
      (bind _asbm_character_base (Utilities|Casting|CastToBM_CharacterBase (Utilities|Array|Get(acopy) _outactor)))
      (Development|PrintString (Utilities|String|Append "Enemy Name=" (.PlayerName (Utilities|Struct|BreakPlayerInfo (Variables|/Script/BuddyMan.BM_PlayerStateBase|GetPlayerInfo (Variables|/Script/BuddyMan.BM_CharacterBase|GetCurPlayerState _asbm_character_base))))))
      (GameplayEffects|ApplyGameplayEffectToTarget :self (.abilitysystemcomponent (Ability|GetActorInfo)) :GameplayEffectClass "/Game/BuddyMan/Ability/GE/GE_BeHit.GE_BeHit_C" :Target (Ability|GetAbilitySystemComponent _asbm_character_base))
      (Ability|SendGameplayEventtoActor _asbm_character_base "(TagName=\"Ability.BeHit\")" (Utilities|Struct|MakeGameplayEventData "(TagName=\"Ability.BeHit\")" (Ability|GetOwningActorfromActorInfo))))))

(event Ability|EventOnEndAbility
  (params (bWasCancelled :type Boolean)))

(fn InitAbilityParam)

(fn FindNearbyEnemy
  (bind _returnvalue (Ability|GetOwningActorfromActorInfo))
  (bind _returnvalue_2 (Transformation|GetActorLocation _returnvalue))
  (Utilities|Array|Clear (Variables|Default|GetHitActors))
  (Utilities|IsValid _returnvalue
    (:Is%20Valid
      (bind _outhits (Class|KismetSystemLibrary|BoxTraceMultiforObjects _returnvalue_2 (+ _returnvalue_2 (* (Transformation|GetActorForwardVector _returnvalue) (Variables|Default|GetDistance))) "100.000000,100.000000,100.000000" "0, 0, 0" (Variables|Default|GetObjectTypes) false 0 "None" true))
      (for _array_element _outhits
        (if (not (Utilities|Array|ContainsItem (Variables|Default|GetHitActors) (.HitActor (Collision|BreakHitResult _array_element))))
          (Utilities|Array|Add (Variables|Default|GetHitActors) (.HitActor (Collision|BreakHitResult _array_element)))))
      (return (Variables|Default|GetHitActors)))))

(fn CalcEnemyDirection
  (params (EnemyActor :type Actor%20Object%20Reference))
  (bind _returnvalue (Ability|GetOwningActorfromActorInfo))
  (if (< (Math|Vector|DotProduct (Transformation|GetActorRightVector _returnvalue) (- (Transformation|GetActorLocation EnemyActor) (Transformation|GetActorLocation _returnvalue))) 0.0)
    (return true)
    (else
      (return false))))

(fn InitCurMontagetbyEnemySide
  (params (bIsLeftSide :type Boolean))
  (bind _asbm_character_base (Utilities|Casting|CastToBM_CharacterBase (Ability|GetOwningActorfromActorInfo)))
  (switch Utilities|FlowControl|Switch|SwitchonECharacterType (Utilities|Enum|ByteToEnumECharacterType (Math|Conversions|ToByte(Integer) (.playertype (Variables|/Script/BuddyMan.BM_PlayerStateBase|GetPlayerInfo (Variables|/Script/BuddyMan.BM_CharacterBase|GetCurPlayerState _asbm_character_base)))))
    (:Ghoul
      (if bIsLeftSide
        (Variables|Default|SetCurMontage (Variables|Default|GetLeft_Attack_Ghoul))
        (else
          (Variables|Default|SetCurMontage (Variables|Default|GetRight_AttackGhoul)))))
    (:Zombie
      (if bIsLeftSide
        (Variables|Default|SetCurMontage (Variables|Default|GetLeft_Attack_Zombie))
        (else
          (Variables|Default|SetCurMontage (Variables|Default|GetRight_Attack_Zombie)))))))

(fn RotatetoEnemy
  (params (Enemy :type Actor%20Object%20Reference))
  (bind _returnvalue (Ability|GetOwningActorfromActorInfo))
  (bind _returnvalue_2 (Transformation|GetActorLocation Enemy))
  (bind (_x _y) (Class|KismetMathLibrary|BreakVector3f _returnvalue_2))
  (bind _returnvalue_3 (Transformation|GetActorLocation _returnvalue))
  (Transformation|SetActorRotation _returnvalue (Math|Rotator|FindLookatRotation _returnvalue_3 (Math|Vector|MakeVector _x _y (.Z (Math|Vector|BreakVector _returnvalue_3))))))