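; Base player character Blueprint that configures itself from its player state and handles basic move and look input.
; When character info changes, a valid player state drives character type, mesh, capsule-height offsets, name/HP widget and spring-arm camera.
; Camera and anim-class lookups index arrays by PlayerType minus one, though InitAnimBP is not called here.
; GetModuleName returns a script module path, suggesting UnLua-style binding; HP display uses a fixed placeholder value.
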(event Custom|CustomEvent_0
  (bind _curplayerstate (Variables|Default|GetCurPlayerState))
  (Development|PrintString "CharacterInfo change....")
  (Utilities|IsValid _curplayerstate
    (:Is%20Valid
      (Development|PrintString "CurPlayerState is not not not null.....")
      (if (> (Variables|/Script/Engine.PlayerState|GetPlayerId _curplayerstate) 0)
        (Variables|Default|SetCharacterType (Utilities|Enum|ByteToEnumECharacterType (Math|Conversions|ToByte(Integer) (.playertype (Variables|/Script/BuddyMan.BM_PlayerStateBase|GetPlayerInfo _curplayerstate)))))
        (Class|BMCharacterBase|InitMesh)
        (Class|BMCharacterBase|InitHeight)
        (CallFunction|InitCharacterAttrHeight)
        (CallFunction|UpdateAttr)
        (CallFunction|InitCamera)))
    (:Is%20Not%20Valid
      (Development|PrintString "CurPlayerState is null....."))))

(event EventBeginPlay
  (Variables|/Script/Engine.PlayerController|SetbShowMouseCursor (Game|GetPlayerController 0) true)
  (EventDispatchers|BindEventtoOnCharacterInfoChange (delegate Custom|CustomEvent_0)))

(event Collision|EventActorBeginOverlap
  (params (OtherActor :type Actor%20Object%20Reference)))

(event EventTick
  (params (DeltaSeconds :type Float%20%28single-precision%29))
  (Utilities|IsValid (Variables|Default|GetCurPlayerState)))

(event EventPossessed
  (params (NewController :type Controller%20Object%20Reference))
  (Development|PrintString "Event Processed...."))

(event Input|AxisEvents|InputAxisMoveForward/Backward
  (params (AxisValue :type Float%20%28single-precision%29))
  (Pawn|Input|AddMovementInput (Math|Vector|GetForwardVector (Pawn|GetControlRotation :!class /Script/Engine.Pawn)) AxisValue false))

(event Input|AxisEvents|InputAxisMoveRight/Left
  (params (AxisValue :type Float%20%28single-precision%29))
  (Pawn|Input|AddMovementInput (Math|Vector|GetRightVector (Pawn|GetControlRotation :!class /Script/Engine.Pawn)) AxisValue false))

(event Input|AxisEvents|InputAxisTurnRight/LeftMouse
  (params (AxisValue :type Float%20%28single-precision%29))
  (Pawn|Input|AddControllerYawInput AxisValue))

(event Input|AxisEvents|InputAxisLookUp/DownMouse
  (params (AxisValue :type Float%20%28single-precision%29))
  (Pawn|Input|AddControllerPitchInput AxisValue))

(fn ConstructionScript)

(fn InitCharacterAttrHeight
  (bind _curplayerstate (Variables|Default|GetCurPlayerState))
  (bind _playerinfo (Variables|/Script/BuddyMan.BM_PlayerStateBase|GetPlayerInfo _curplayerstate))
  (bind (_id _playername _playertype _halfheight) (Utilities|Struct|BreakPlayerInfo _playerinfo))
  (bind _returnvalue (* _halfheight -1.0))
  (bind _returnvalue_2 (* _halfheight 2.0))
  (bind _returnvalue_3 (Math|Vector|MakeVector 0.0 0.0 _returnvalue))
  (bind _returnvalue_4 (Math|Vector|MakeVector 0.0 0.0 _returnvalue_2))
  (Development|PrintString (Utilities|String|Append "HalfHeight=" (Utilities|String|ToString(Float) _halfheight) ",MeshLocation=" (Utilities|String|ToString(Vector) _returnvalue_3) ",AttrWidgetLocation=" (Utilities|String|ToString(Vector) _returnvalue_4) ",PlayerName=" _playername))
  (Transformation|SetRelativeLocation (Variables|Default|GetAttrWidget) _returnvalue_4 false false)
  (Class|Character|CacheInitialMeshOffset _returnvalue_3 (Math|Rotator|MakeRotator 0.0 0.0 -9e+01)))

(fn UpdateAttr
  (bind _curplayerstate (Variables|Default|GetCurPlayerState))
  (bind _returnvalue (PlayerState|GetPlayerName _curplayerstate))
  (bind _asup_player_attr (Utilities|Casting|CastToUP_PlayerAttr (UserInterface|GetUserWidgetObject (Variables|Default|GetAttrWidget))))
  (Default|UpdateName _asup_player_attr _returnvalue)
  (Development|PrintString (Utilities|String|Append "OnSetText Name=" _returnvalue))
  (Default|UpdateHp _asup_player_attr (- (.PlayerType (Utilities|Struct|BreakPlayerInfo (Variables|/Script/BuddyMan.BM_PlayerStateBase|GetPlayerInfo _curplayerstate))) 1) 3e+01))

(fn InitAnimBP
  (bind _curplayerstate (Variables|Default|GetCurPlayerState))
  (Utilities|IsValid _curplayerstate
    (:Is%20Valid
      (if (> (Variables|/Script/Engine.PlayerState|GetPlayerId _curplayerstate) 0)
        (bind _returnvalue (Class|BuddyManBlueprintLibrary|GetAnimBlueprintGeneratedClass (Utilities|Array|Get(acopy) (Variables|Default|GetAnimClasses) (- (.PlayerType (Utilities|Struct|BreakPlayerInfo (Variables|/Script/BuddyMan.BM_PlayerStateBase|GetPlayerInfo _curplayerstate))) 1))))
        (Class|SkeletalMeshComponent|SetAnimClass (Variables|Character|GetMesh) _returnvalue)))))

(fn InitCamera
  (bind _curplayerstate (Variables|Default|GetCurPlayerState))
  (bind _springarm (Variables|Default|GetSpringArm))
  (bind _playerinfo (Variables|/Script/BuddyMan.BM_PlayerStateBase|GetPlayerInfo _curplayerstate))
  (bind _returnvalue (- (.playertype _playerinfo) 1))
  (Utilities|IsValid _curplayerstate
    (:Is%20Valid
      (Variables|/Script/Engine.SpringArmComponent|SetTargetArmLength _springarm (Math|Conversions|ToFloat(Integer) (Utilities|Array|Get(acopy) (Variables|Default|GetSpringArmLength) _returnvalue)))
      (Variables|/Script/Engine.SpringArmComponent|SetTargetOffset _springarm (Math|Vector|MakeVector 0.0 0.0 (Math|Conversions|ToFloat(Integer) (Utilities|Array|Get(acopy) (Variables|Default|GetSpringArmOffsetZ) _returnvalue)))))))

(fn GetModuleName
  (return "BuddyMain.Blueprints.Character.BP_Character_Base"))